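; Telekinesis target object that the player can highlight, pull toward their telekinesis source, and launch at a destination.
; Pull plays a lift timeline, then disables gravity; Tick applies mass-scaled impulses to reach the player with random jitter, or the push target.
; While active it attracts nearby BP_PhysicsObjects via an overlap sphere and feeds mesh socket locations to Niagara trails.
; A hit while pushed restores physics, bounces and spawns sparks.
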(event OnComponentHit(StaticMesh)
  (params (HitComponent :type Primitive%20Component%20Object%20Reference) (OtherActor :type Actor%20Object%20Reference) (OtherComp :type Primitive%20Component%20Object%20Reference) (NormalImpulse :type Vector :default "0, 0, 0") (Hit :type Hit%20Result%20Structure%20%28by%20ref%29))
  ;[1 1 1] On hit triggers
  (CallFunction|Hit NormalImpulse))

(event OnComponentBeginOverlap(AttractionField)
  (params (OverlappedComponent :type Primitive%20Component%20Object%20Reference) (OtherActor :type Actor%20Object%20Reference) (OtherComp :type Primitive%20Component%20Object%20Reference) (OtherBodyIndex :type Integer) (bFromSweep :type Boolean) (SweepResult :type Hit%20Result%20Structure%20%28by%20ref%29))
  ;[1 1 1] Overlaps
  (bind _asbp_physics_object (Utilities|Casting|CastToBP_PhysicsObject OtherActor))
  (CallFunction|AddPhysicsObjects _asbp_physics_object))

(event OnComponentEndOverlap(AttractionField)
  (params (OverlappedComponent :type Primitive%20Component%20Object%20Reference) (OtherActor :type Actor%20Object%20Reference) (OtherComp :type Primitive%20Component%20Object%20Reference) (OtherBodyIndex :type Integer))
  ;[1 1 1] Overlaps
  (bind _asbp_physics_object (Utilities|Casting|CastToBP_PhysicsObject OtherActor))
  (CallFunction|RemovePhysicsObject _asbp_physics_object))

(event Custom|LiftOff
  (bind _returnvalue (Transformation|GetActorLocation))
  ;[1 1 1] Lift off logic
  (Audio|PlaySound2D "/Game/Telekinesis/Sounds/A_LiftOff.A_LiftOff" 1.0 1.0 0.0 0 0)
  (CallFunction|Highlight false)
  (Components|Activation|Activate (Variables|Default|GetNiagara) false)
  (Variables|Movement|SetLiftStart _returnvalue)
  (Variables|Movement|SetLiftTarget (+ _returnvalue (Math|Vector|MakeVector 0.0 0.0 (Variables|Movement|GetLiftHeight))))
  (bind _height (Timeline|Lift PlayFromStart)
    (:Update
      (Transformation|SetActorLocation (Math|Vector|Lerp(Vector) (Variables|Movement|GetLiftStart) (Variables|Movement|GetLiftTarget) _height) false false))
    (:Finished
      (CallFunction|InitializePull))))

(event Custom|StopLifting
  ;[1 1 1] Lift off logic
  (bind _height (Timeline|Lift Stop)
    (:Update
      (Transformation|SetActorLocation (Math|Vector|Lerp(Vector) (Variables|Movement|GetLiftStart) (Variables|Movement|GetLiftTarget) _height) false false))
    (:Finished
      (CallFunction|InitializePull))))

(event EventBeginPlay
  ;[1 1 1] BeingPlay
  (CallFunction|ActivateTrails))

(event EventHighlight
  (params (bHighlight :type Boolean))
  ;[1 1 1] Outline visibility
  (if (Utilities|Enum|Equal(Enum) (Variables|Movement|GetState) "NewEnumerator0")
    (Rendering|SetRenderCustomDepth (Variables|Default|GetStaticMesh) bHighlight)))

(event EventPush
  (params (Destination :type Vector :default "0, 0, 0"))
  ;[1 1 1] Push logic
  (Variables|Movement|SetPushTarget Destination)
  (Variables|Movement|SetState "NewEnumerator2")
  (CallFunction|DisablePhysicsObjectCollision)
  (CallFunction|StopLifting)
  (CallFunction|SpawnSparks (Math|Vector|GetUnitDirection(Vector) (Transformation|GetActorLocation) (Variables|Movement|GetPushTarget)))
  (Components|Activation|Deactivate (Variables|Default|GetWind))
  (Audio|PlaySound2D "/Game/Telekinesis/Sounds/A_Push.A_Push" 1.0 1.0 0.0 0 0))

(event EventTick
  (params (DeltaSeconds :type Float%20%28single-precision%29))
  ;[1 1 1] Tick
  (switch Utilities|FlowControl|Switch|SwitchonE_Status (Variables|Movement|GetState)
    (:NewEnumerator1
      (CallFunction|ReachCharacter))
    (:NewEnumerator2
      (CallFunction|ReachTarget)))
  (CallFunction|FeedSocketLocationstoNS)
  (CallFunction|AttractPhysicsObject))

(fn ConstructionScript
  (Transformation|SetWorldScale3D (Variables|Default|GetAttractionField) "1.000000,1.000000,1.000000"))

(fn ReachCharacter
  (Physics|AddImpulse (Variables|Default|GetStaticMesh) (* (Math|Vector|ClampVectorSize (- (Transformation|GetWorldLocation (Variables|/Game/Telekinesis/Core/BP_ControlCharacter.BP_ControlCharacter_C|GetTelekinesisSource (Variables|Default|GetPlayerCharacter))) (Transformation|GetActorLocation)) 0.0 1e+03) (Math|Float|MapRangeClamped (Physics|GetMass (Variables|Default|GetStaticMesh)) (Variables|Movement|GetMassMinClamp) (Variables|Movement|GetMassMaxClamp) (Variables|Movement|GetMinSpeedMultiplier) (Variables|Movement|GetMaxSpeedMultiplier))) "None" true)
  (CallFunction|Jitter))

(fn ReachTarget
  (Physics|AddImpulse (Variables|Default|GetStaticMesh) (* (Math|Vector|GetUnitDirection(Vector) (Transformation|GetActorLocation) (Variables|Movement|GetPushTarget)) (* (Math|Float|MapRangeClamped (Physics|GetMass (Variables|Default|GetStaticMesh)) (Variables|Movement|GetMassMinClamp) (Variables|Movement|GetMassMaxClamp) (Variables|Movement|GetMinSpeedMultiplier) (Variables|Movement|GetMaxSpeedMultiplier)) (Variables|Movement|GetPushSpeed))) "None" true))

(fn FeedSocketLocationstoNS
  (if (!= (Utilities|Array|Length (Transformation|GetAllSocketNames (Variables|Default|GetStaticMesh))) 0)
    (for (_array_element _array_index) (Transformation|GetAllSocketNames (Variables|Default|GetStaticMesh))
      (Effects|Components|ParticleSystem|SetVectorParameter (Variables|Default|GetNiagara) (Utilities|String|StringToName (Utilities|String|Append "Location" (Utilities|String|ToString(Integer) _array_index))) (Transformation|GetSocketLocation (Variables|Default|GetStaticMesh) _array_element)))
    (else
      (Effects|Components|ParticleSystem|SetVectorParameter (Variables|Default|GetNiagara) "Location0" (Transformation|GetActorLocation)))))

(fn ActivateTrails
  (if (!= (Utilities|Array|Length (Transformation|GetAllSocketNames (Variables|Default|GetStaticMesh))) 0)
    (for (_ _array_index) (Transformation|GetAllSocketNames (Variables|Default|GetStaticMesh))
      (Effects|Components|ParticleSystem|SetFloatParameter (Variables|Default|GetNiagara) (Utilities|String|StringToName (Utilities|String|Append "Spawn" (Utilities|String|ToString(Integer) _array_index))) (Variables|Default|GetSpawnRate)))
    (else
      (Effects|Components|ParticleSystem|SetFloatParameter (Variables|Default|GetNiagara) "Spawn0" (Variables|Default|GetSpawnRate)))))

(fn Hit
  (params (Impulse :type Vector))
  (bind _staticmesh (Variables|Default|GetStaticMesh))
  (if (Utilities|Enum|Equal(Enum) (Variables|Movement|GetState) "NewEnumerator2")
    (Physics|SetEnableGravity _staticmesh true)
    (Class|PrimitiveComponent|SetLinearDamping _staticmesh 0.01)
    (Variables|Movement|SetState "NewEnumerator0")
    (Class|PrimitiveComponent|SetAllPhysicsLinearVelocity (Variables|Default|GetStaticMesh) "0, 0, 0" false)
    (Physics|AddImpulse (Variables|Default|GetStaticMesh) (* Impulse (Variables|Movement|GetBounciness)) "None" false)
    (Components|Activation|Deactivate (Variables|Default|GetNiagara))
    (CallFunction|SpawnSparks Impulse)))

(fn InitializePull
  (bind _staticmesh (Variables|Default|GetStaticMesh))
  (Class|PrimitiveComponent|AddAngularImpulseinDegrees (Variables|Default|GetStaticMesh) (* (Transformation|GetActorUpVector (Variables|Default|GetPlayerCharacter)) 8e+02) "None" true)
  (Components|Activation|Activate (Variables|Default|GetWind) true)
  (CallFunction|DetectPhysicsObjects)
  (Physics|SetEnableGravity _staticmesh false)
  (Class|PrimitiveComponent|SetLinearDamping _staticmesh 2e+01)
  (Variables|Movement|SetState "NewEnumerator1"))

(fn SpawnSparks
  (params (Impulse :type Vector))
  (bind _returnvalue (Niagara|SpawnSystematLocation "/Game/Telekinesis/VFX/NS_Sparks.NS_Sparks" (Transformation|GetActorLocation)))
  (Effects|Components|ParticleSystem|SetVectorParameter _returnvalue "Direction" (Math|Vector|Normalize Impulse)))

(fn AttractPhysicsObject
  (for _array_element (Variables|Default|GetPhysicsObjects)
    (Default|AttractForce _array_element (Math|Vector|GetUnitDirection(Vector) (Transformation|GetActorLocation _array_element) (Transformation|GetActorLocation)))))

(fn DisablePhysicsObjectCollision
  (for _array_element (Variables|Default|GetPhysicsObjects)
    (Collision|SetCollisionResponsetoChannel (Variables|/Game/Telekinesis/Core/BP_PhysicsObject.BP_PhysicsObject_C|GetStaticMesh _array_element) "ECC_GameTraceChannel1" "ECR_Ignore")))

(fn AddPhysicsObjects
  (params (PhysicsObject :type BP%20Physics%20Object%20Object%20Reference%20%28by%20ref%29))
  (bind _staticmesh (Variables|/Game/Telekinesis/Core/BP_PhysicsObject.BP_PhysicsObject_C|GetStaticMesh PhysicsObject))
  (Utilities|Array|Add (Variables|Default|GetPhysicsObjects) PhysicsObject)
  (Physics|SetEnableGravity _staticmesh false)
  (Class|PrimitiveComponent|SetLinearDamping _staticmesh 1e+01)
  (Collision|SetCollisionResponsetoChannel _staticmesh "ECC_GameTraceChannel1" "ECR_Block"))

(fn RemovePhysicsObject
  (params (PhysicsObject :type BP%20Physics%20Object%20Object%20Reference%20%28by%20ref%29))
  (bind _staticmesh (Variables|/Game/Telekinesis/Core/BP_PhysicsObject.BP_PhysicsObject_C|GetStaticMesh PhysicsObject))
  (Utilities|Array|RemoveItem (Variables|Default|GetPhysicsObjects) PhysicsObject)
  (Physics|SetEnableGravity _staticmesh true)
  (Class|PrimitiveComponent|SetLinearDamping _staticmesh 0.01))

(fn DetectPhysicsObjects
  (bind _returnvalue (Transformation|GetActorLocation))
  (bind _outhits (Collision|MultiSphereTraceForObjects _returnvalue _returnvalue (Components|Sphere|GetScaledSphereRadius (Variables|Default|GetAttractionField)) (Utilities|Array|MakeArray "ObjectTypeQuery2") false 0 "None"))
  (for _array_element _outhits
    (bind _asbp_physics_object (Utilities|Casting|CastToBP_PhysicsObject (.hitactor _array_element)))
    (CallFunction|AddPhysicsObjects _asbp_physics_object)))

(fn Jitter
  (bind _output_get (Variables|Default|SetJitterCounter (+ (Variables|Default|GetJitterCounter) 1)))
  (if (== _output_get (Variables|Default|GetJitterFrameTime))
    (Variables|Default|SetJitterCounter 0)
    (Variables|Default|SetJitterFrameTime (Math|Random|RandomIntegerinRange 20 30))
    (Physics|AddImpulse (Variables|Default|GetStaticMesh) (* (Math|Random|RandomUnitVector) 2e+02) "None" true)))

(fn Pull
  (params (PlayerCharacter :type BP%20Control%20Character%20Object%20Reference))
  (Variables|Default|SetPlayerCharacter PlayerCharacter)
  (CallFunction|LiftOff)
  (return))